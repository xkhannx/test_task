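; BP_Cat is a cat actor that travels in a straight line to a destination, colored and moving according to its nest index.
; SpawnCat tints the mesh and Niagara effect red, green or blue, stores the direction and starts sounds.
; Tick selects the gait: steady, stop-and-go, or forward-and-backtrack on a timer.
; IsDone detects overshoot with a dot product, snaps to the destination, plays end effects and destroys the cat.
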(event `self.ReceiveBeginPlay`)

(event `self.ReceiveTick`
  (params (DeltaSeconds :type "Float (single-precision)"))
  (if (`self.Started`)
    (set `self.dt` DeltaSeconds)
    (switch `int` (`self.Cat Index`)
      (:`0`
        (bind _returnvalue (`self.Walk 1`))
        (`self.K2_SetActorLocation` _returnvalue))
      (:`1`
        (bind _returnvalue_2 (`self.Walk 2`))
        (`self.K2_SetActorLocation` _returnvalue_2))
      (:`2`
        (bind _returnvalue_3 (`self.Walk 3`))
        (`self.K2_SetActorLocation` _returnvalue_3)))
    (`self.Is Done`)))

(fn `Is Done`
  (bind _end_pos (`self.End Pos`))
  (if (< (`KismetMathLibrary.Dot_VectorVector` (- (`self.End Pos`) (`self.K2_GetActorLocation`)) (`self.Direction`)) 0.0)
    (`self.K2_SetActorLocation` (`self.End Pos`))
    (set `self.Started` false)
    (`GameplayStatics.PlaySoundAtLocation` "/Game/FX/meow_end.meow_end" _end_pos (struct) 1.0 1.0 0.0 null null null)
    (`NiagaraFunctionLibrary.SpawnSystemAtLocation` "/Game/FX/VFX_End_System.VFX_End_System" _end_pos)
    (`self.K2_DestroyActor`)))

(fn `Spawn Cat`
  (params (Destination :type "Vector Structure") (`Nest Index` :type Integer))
  (bind _niagara (`self.Niagara`))
  (bind _staticmesh (`self.StaticMesh`))
  (set `self.End Pos` Destination)
  ;[1 1 1] Set up materials
  (set `self.Cat Index` `Nest Index`)
  (bind _returnvalue (`PrimitiveComponent.CreateDynamicMaterialInstance` _staticmesh 0 "/Game/Models/Cat/Cat_mat.Cat_mat" "None"))
  (`PrimitiveComponent.SetMaterial` _staticmesh 0 _returnvalue)
  (switch `int` `Nest Index`
    (:`0`
      (`MaterialInstanceDynamic.SetVectorParameterValue` _returnvalue "CatColor" (make `LinearColor` 1.0 0.0 0.0 1.0))
      (`NiagaraComponent.SetVariableLinearColor` _niagara "User.SpawnVFXColor" (make `LinearColor` 1.0 0.0 0.0 1.0)))
    (:`1`
      (`MaterialInstanceDynamic.SetVectorParameterValue` _returnvalue "CatColor" (make `LinearColor` 0.0 1.0 0.0 1.0))
      (`NiagaraComponent.SetVariableLinearColor` _niagara "User.SpawnVFXColor" (make `LinearColor` 0.0 1.0 0.0 1.0)))
    (:`2`
      (`MaterialInstanceDynamic.SetVectorParameterValue` _returnvalue "CatColor" (make `LinearColor` 0.0 0.0 1.0 1.0))
      (`NiagaraComponent.SetVariableLinearColor` _niagara "User.SpawnVFXColor" (make `LinearColor` 0.0 0.0 1.0 1.0))))
  (set `self.Started` true)
  (set `self.Direction` (`KismetMathLibrary.Normal` (- (`self.End Pos`) (`self.K2_GetActorLocation`))))
  (set `self.MovingForward` true)
  ;[1 1 1] Play sounds
  (`GameplayStatics.PlaySoundAtLocation` "/Game/FX/meow_start.meow_start" (`self.K2_GetActorLocation`) (struct) 2.0 1.0 0.0 null null null)
  (bind _returnvalue_2 (`GameplayStatics.SpawnSoundAttached` "/Game/FX/walking.walking" (`self.StaticMesh`) "None" (0.0 0.0 0.0) (struct) "KeepRelativeOffset" true 0.2 1.0 0.0 null null))
  (set `self.WalkingSound` _returnvalue_2))

(fn `UserConstructionScript`)

(fn `Walk 1`
  (returns (ReturnValue :type "Vector Structure"))
  (return (+ (`self.K2_GetActorLocation`) (* (`self.Direction`) (* (`self.Move Speed`) (`self.dt`))))))

(fn `Walk 2`
  (returns (ReturnValue :type "Vector Structure"))
  (bind _output_get (set `self.CurTime` (+ (`self.CurTime`) (`self.dt`))))
  (if (`self.MovingForward`)
    (if (> _output_get 1.0)
      (set `self.CurTime` 0.0)
      (set `self.MovingForward` false))
    (elif (> _output_get 0.5)
      (set `self.CurTime` 0.0)
      (set `self.MovingForward` true)
      (else
        (set `self.dt` 0.0))))
  (return (+ (`self.K2_GetActorLocation`) (* (`self.Direction`) (* (`self.Move Speed`) (`self.dt`))))))

(fn `Walk 3`
  (returns (ReturnValue :type "Vector Structure"))
  (bind _output_get (set `self.CurTime` (+ (`self.CurTime`) (`self.dt`))))
  (if (`self.MovingForward`)
    (if (> _output_get 1.0)
      (set `self.CurTime` 0.0)
      (set `self.MovingForward` false))
    (elif (> _output_get 0.5)
      (set `self.CurTime` 0.0)
      (set `self.MovingForward` true)
      (else
        (set `self.dt` (* (`self.dt`) -1.0)))))
  (return (+ (`self.K2_GetActorLocation`) (* (`self.Direction`) (* (`self.Move Speed`) (`self.dt`))))))